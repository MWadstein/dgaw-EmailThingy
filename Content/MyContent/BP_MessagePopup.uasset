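; BP_MessagePopup is an interactable world object that shows a message popup widget.
; Overlapping its MessageCollider reveals a TextRender and enables interaction, while leaving hides the text and closes any open popup.
; InteractwithObject toggles a MessagePopup widget fed by the Messages variable, switching input mode and mouse cursor to match.
; The widget's ED_CloseClicked dispatcher calls back into the same toggle to close it.
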(event `/Game/MyContent/BP_EmailPopup.ReceiveBeginPlay`
  (`SceneComponent.SetVisibility` (`self.TextRender`) false false))

(event `self.MessageCollider.OnComponentBeginOverlap`
  (params (OtherActor :type "Actor Object Reference") (OtherComp :type "PrimitiveComponent Object Reference") (OtherBodyIndex :type Integer) (bFromSweep :type Boolean) (SweepResult :type "HitResult Structure (by ref)"))
  (`SceneComponent.SetVisibility` (`self.TextRender`) true false)
  (set `self.Interactable` true))

(event `self.MessageCollider.OnComponentEndOverlap`
  (params (OtherActor :type "Actor Object Reference") (OtherComp :type "PrimitiveComponent Object Reference") (OtherBodyIndex :type Integer))
  (bind _returnvalue (`GameplayStatics.GetPlayerController` 0))
  (`SceneComponent.SetVisibility` (`self.TextRender`) false false)
  (set `self.Interactable` false)
  (if (not (== null null))
    (`Widget.RemoveFromParent` (`self.Widget`))
    (set `self.Widget` null)
    (`WidgetBlueprintLibrary.SetInputMode_GameOnly` _returnvalue)
    (set `PlayerController.bShowMouseCursor` false _returnvalue)))

(event `/Game/MyContent/Interactable.InteractWithObject`
  (bind _returnvalue (`GameplayStatics.GetPlayerController` 0))
  (bind _returnvalue_2 (`GameplayStatics.GetPlayerController` 0))
  (if (== (`self.Widget`) null)
    (if (`self.Interactable`)
      (bind _returnvalue_3 (`|CreateWidget` "/Game/MyContent/MessagePopup.MessagePopup_C" null (`self.Messages`)))
      (bind _output_get (set `self.Widget` _returnvalue_3))
      (`UserWidget.AddToViewport` _output_get 0)
      (`WidgetBlueprintLibrary.SetInputMode_UIOnlyEx` _returnvalue)
      (set `PlayerController.bShowMouseCursor` true _returnvalue)
      (add `/Game/MyContent/MessagePopup.ED_CloseClicked` (`self.Widget`) (delegate `ED_CloseClicked_Event_0`)))
    (else
      (`Widget.RemoveFromParent` (`self.Widget`))
      (set `self.Widget` null)
      (`WidgetBlueprintLibrary.SetInputMode_GameOnly` _returnvalue_2)
      (set `PlayerController.bShowMouseCursor` false _returnvalue_2))))

(event `ED_CloseClicked_Event_0`
  (`self.InteractWithObject`))

(fn `UserConstructionScript`)